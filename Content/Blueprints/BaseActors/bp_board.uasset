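; Card game board actor that detects cards landing in Player 1's equip, character, power, play and protection slots.
; BeginPlay caches the player UI from the game instance and stores twelve equip slot transforms.
; Slot overlaps (only the first equip slot is wired; play ignores in-hand cards) stop the card and flag occupancy.
; They then lock the card and call hand reassignment with its former hand index.
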(event `Trigger Hand Re-assignment for Player`
  (params (`Card Being Played` :type "Actor Object Reference"))
  ;[1 1 1] Trigger Hand Re-assignment for Player
  (bind _asbp_game_instance (cast `/Game/GameMode/bp_GameInstance` (`GameplayStatics.GetGameInstance`)))
  (bind _asbp_card (cast `/Game/Blueprints/BaseActors/bp_Card` `Card Being Played`))
  (set `/Game/Blueprints/BaseActors/bp_Card.Possition Locked` true _asbp_card)
  (`self.Trigger Hand Re-assignment` (`KismetArrayLibrary.Array_Find` (`/Game/GameMode/bp_GameInstance.Player 1's Location in Hand` _asbp_game_instance) (`/Game/Blueprints/BaseActors/bp_Card.Defult Location` _asbp_card))))

(event `self.obj_p1_EquipSlot_1.OnComponentBeginOverlap`
  (params (OverlappedComponent :type "PrimitiveComponent Object Reference") (OtherActor :type "Actor Object Reference") (OtherComp :type "PrimitiveComponent Object Reference") (OtherBodyIndex :type Integer) (bFromSweep :type Boolean) (SweepResult :type "HitResult Structure (by ref)"))
  ;[1 1 1] Player 1 Equip Card Check and Assignment
  (bind _asbp_card (cast `/Game/Blueprints/BaseActors/bp_Card` OtherActor))
  (set `/Game/Blueprints/BaseActors/bp_Card.In Motion` false _asbp_card)
  (set `self.P1 Eslot Space Occupied_0` true)
  (`self.Trigger Hand Re-assignment for Player` _asbp_card)
  (`KismetSystemLibrary.PrintString` "Equip" true true (struct :`R` 0.213542 :`G` 0.016647 :`A` 1.0)))

(event `self.obj_p1_CharacterSlot.OnComponentBeginOverlap`
  (params (OverlappedComponent :type "PrimitiveComponent Object Reference") (OtherActor :type "Actor Object Reference") (OtherComp :type "PrimitiveComponent Object Reference") (OtherBodyIndex :type Integer) (bFromSweep :type Boolean) (SweepResult :type "HitResult Structure (by ref)"))
  ;[1 1 1] Player 1 Character Card Check
  (bind _asbp_card (cast `/Game/Blueprints/BaseActors/bp_Card` OtherActor))
  (set `/Game/Blueprints/BaseActors/bp_Card.In Motion` false _asbp_card)
  (set `self.P1 Cslot Space Occupied` true)
  (`self.Trigger Hand Re-assignment for Player` _asbp_card)
  (`KismetSystemLibrary.PrintString` "Chracter" true true (struct :`G` 0.020776 :`B` 0.213542 :`A` 1.0)))

(event `self.ReceiveBeginPlay`
  (bind _p1_equipcardlocations (`self.P1 EquipCardLocations`))
  (bind _p1_equip_card_slot_on_board (`self.P1 Equip Card Slot on Board`))
  ;[1 1 1] Equip Card Assignemnt (P1)
  (bind _asbp_game_instance (cast `/Game/GameMode/bp_GameInstance` (`GameplayStatics.GetGameInstance`)))
  (set `self.P1 User Interface` (`/Game/GameMode/bp_GameInstance.P1 UserInterface` _asbp_game_instance))
  (while (< _p1_equip_card_slot_on_board 12)
    (switch `int` _p1_equip_card_slot_on_board
      (:`0`
        (`KismetArrayLibrary.Array_Add` _p1_equipcardlocations (`SceneComponent.K2_GetComponentToWorld` (`self.obj_p1_EquipSlot_1`))))
      (:`1`
        (`KismetArrayLibrary.Array_Add` _p1_equipcardlocations (`SceneComponent.K2_GetComponentToWorld` (`self.obj_p1_EquipSlot_2`))))
      (:`2`
        (`KismetArrayLibrary.Array_Add` _p1_equipcardlocations (`SceneComponent.K2_GetComponentToWorld` (`self.obj_p1_EquipSlot_3`))))
      (:`3`
        (`KismetArrayLibrary.Array_Add` _p1_equipcardlocations (`SceneComponent.K2_GetComponentToWorld` (`self.obj_p1_EquipSlot_4`))))
      (:`4`
        (`KismetArrayLibrary.Array_Add` _p1_equipcardlocations (`SceneComponent.K2_GetComponentToWorld` (`self.obj_p1_EquipSlot_5`))))
      (:`5`
        (`KismetArrayLibrary.Array_Add` _p1_equipcardlocations (`SceneComponent.K2_GetComponentToWorld` (`self.obj_p1_EquipSlot_6`))))
      (:`6`
        (`KismetArrayLibrary.Array_Add` _p1_equipcardlocations (`SceneComponent.K2_GetComponentToWorld` (`self.obj_p1_EquipSlot_7`))))
      (:`7`
        (`KismetArrayLibrary.Array_Add` _p1_equipcardlocations (`SceneComponent.K2_GetComponentToWorld` (`self.obj_p1_EquipSlot_8`))))
      (:`8`
        (`KismetArrayLibrary.Array_Add` _p1_equipcardlocations (`SceneComponent.K2_GetComponentToWorld` (`self.obj_p1_EquipSlot_9`))))
      (:`9`
        (`KismetArrayLibrary.Array_Add` _p1_equipcardlocations (`SceneComponent.K2_GetComponentToWorld` (`self.obj_p1_EquipSlot_10`))))
      (:`10`
        (`KismetArrayLibrary.Array_Add` _p1_equipcardlocations (`SceneComponent.K2_GetComponentToWorld` (`self.obj_p1_EquipSlot_11`))))
      (:`11`
        (`KismetArrayLibrary.Array_Add` _p1_equipcardlocations (`SceneComponent.K2_GetComponentToWorld` (`self.obj_p1_EquipSlot_12`)))))
    (set `self.P1 Equip Card Slot on Board` (+ (`self.P1 Equip Card Slot on Board`) 1)))
  (set `self.P1 Equip Card Slot on Board` 0))

(event `self.obj_p1_PowerSlot.OnComponentBeginOverlap`
  (params (OverlappedComponent :type "PrimitiveComponent Object Reference") (OtherActor :type "Actor Object Reference") (OtherComp :type "PrimitiveComponent Object Reference") (OtherBodyIndex :type Integer) (bFromSweep :type Boolean) (SweepResult :type "HitResult Structure (by ref)"))
  ;[1 1 1] Player 1 Power Card Check
  (bind _asbp_card (cast `/Game/Blueprints/BaseActors/bp_Card` OtherActor))
  (set `/Game/Blueprints/BaseActors/bp_Card.In Motion` false _asbp_card)
  (set `self.P1 POslot Space Occupied` true)
  (`self.Trigger Hand Re-assignment for Player` _asbp_card)
  (`KismetSystemLibrary.PrintString` "Power" true true (struct :`R` 0.213542 :`G` 0.008463 :`B` 0.177307 :`A` 1.0)))

(event `self.obj_p1_PlaySlot.OnComponentBeginOverlap`
  (params (OverlappedComponent :type "PrimitiveComponent Object Reference") (OtherActor :type "Actor Object Reference") (OtherComp :type "PrimitiveComponent Object Reference") (OtherBodyIndex :type Integer) (bFromSweep :type Boolean) (SweepResult :type "HitResult Structure (by ref)"))
  ;[1 1 1] Player 1 Play Card Check
  (bind _asbp_card (cast `/Game/Blueprints/BaseActors/bp_Card` OtherActor))
  (if (not (`/Game/Blueprints/BaseActors/bp_Card.In Hand` _asbp_card))
    (set `/Game/Blueprints/BaseActors/bp_Card.In Motion` false _asbp_card)
    (set `self.P1 Pslot Space Occupied` true)
    (`self.Trigger Hand Re-assignment for Player` _asbp_card)
    (`KismetSystemLibrary.PrintString` "Play" true true (struct :`G` 0.213542 :`B` 0.124845 :`A` 1.0))))

(event `self.obj_p1_ProtectionSlot.OnComponentBeginOverlap`
  (params (OverlappedComponent :type "PrimitiveComponent Object Reference") (OtherActor :type "Actor Object Reference") (OtherComp :type "PrimitiveComponent Object Reference") (OtherBodyIndex :type Integer) (bFromSweep :type Boolean) (SweepResult :type "HitResult Structure (by ref)"))
  ;[1 1 1] Player 1 Protection Card Check
  (bind _asbp_card (cast `/Game/Blueprints/BaseActors/bp_Card` OtherActor))
  (set `/Game/Blueprints/BaseActors/bp_Card.In Motion` false _asbp_card)
  (set `self.P1 PRslot Space Occupied` true)
  (`self.Trigger Hand Re-assignment for Player` _asbp_card)
  (`KismetSystemLibrary.PrintString` "Proteection" true true (struct :`G` 0.197133 :`B` 0.213542 :`A` 1.0)))

(fn `UserConstructionScript`)