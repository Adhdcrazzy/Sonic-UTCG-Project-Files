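; Player one's deck actor: it builds a card list at start and offers a draw button when clicked.
; On BeginPlay it fills DeckList from the game instance's P1Deck by random picks with replacement, so duplicates can occur, then caches the game instance.
; A click moves Button2 of the P1 user interface near the mouse cursor and makes it visible; the draw itself is not handled here.
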(event `self.ReceiveActorOnClicked`
  (params (ButtonPressed :type "Key Structure"))
  (bind _button_2 (`/Game/Blueprints/Huds/bp_p1_UI.Button_2` (`/Game/GameMode/bp_GameInstance.P1 UserInterface` (`self.Game Instance`))))
  ;[1 1 1] Click to Draw
  (bind _returnvalue (`WidgetLayoutLibrary.GetMousePositionOnViewport`))
  (`Widget.SetRenderTransform` _button_2 (make `WidgetTransform` (`KismetMathLibrary.MakeVector2D` (- (`KismetMathLibrary.BreakVector2D` _returnvalue) 90.0) (- (`.Y` (`KismetMathLibrary.BreakVector2D` _returnvalue)) 50.0))))
  (`Widget.SetVisibility` _button_2 "Visible"))

(event `self.ReceiveBeginPlay`
  ;[1 1 1] Build Deck
  (while (< (`self.Current Card Count`) 31)
    (bind _asbp_game_instance (cast `/Game/GameMode/bp_GameInstance` (`GameplayStatics.GetGameInstance`)))
    (`KismetArrayLibrary.Array_Add` (`self.Deck List`) (`|GetArrayItem` (`/Game/GameMode/bp_GameInstance.P1 Deck` _asbp_game_instance) (`KismetMathLibrary.RandomInteger` 32)))
    (set `self.Current Card Count` (+ (`self.Current Card Count`) 1)))
  (bind _asbp_game_instance_2 (cast `/Game/GameMode/bp_GameInstance` (`GameplayStatics.GetGameInstance`)))
  (set `self.Game Instance` _asbp_game_instance_2))

(fn `UserConstructionScript`)