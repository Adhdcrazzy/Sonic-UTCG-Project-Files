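; Base actor for a card in Player 1's hand, handling hover, selection and movement.
; On spawn it takes an instance ID from the game instance and binds to player and card events that reposition it in the hand.
; Hovering shows a UI close-up and raises the card unless moving or locked; clicking places a button at the cursor.
; That button's press marks the matching card in motion and calls PlayCard, which is empty here.
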(event `self.ReceiveActorEndCursorOver`
  ;[1 1 1] Hover Over Card (End)
  (if (`self.In Motion`)
    _
    (elif (not (`self.Possition Locked`))
      (`KismetSystemLibrary.MoveComponentTo` (`self.obj_Card`) (`self.Defult Location`) (`self.Rotation`)))))

(event `self.obj_Card.OnBeginCursorOver`
  (params (TouchedComponent :type "PrimitiveComponent Object Reference"))
  (bind _closeup (`/Game/Blueprints/Huds/bp_p1_UI.CloseUp` (`self.P1 User Interface`)))
  ;[1 1 1] Hover Over Card (Start)
  ;;[1 1 1] Set Image and Visibility on UI
  (`Image.SetBrush` _closeup (make `SlateBrush` (32.0 32.0) (struct) (struct :`SpecifiedColor` (struct :`R` 1.0 :`G` 1.0 :`B` 1.0 :`A` 1.0) :`ColorUseRule` "UseColor_Specified") (`self.Image for UI`)))
  (`Widget.SetVisibility` _closeup "Visible")
  ;;[1 1 1] Move to Location
  (if (`self.In Motion`)
    _
    (elif (not (`self.Possition Locked`))
      (`KismetSystemLibrary.MoveComponentTo` (`self.obj_Card`) (+ (`self.Defult Location`) (0.0 2.0 1.2)) (`self.Rotation`)))))

(event `Move Card in Hand`
  ;[1 1 1] Move Location In Hand
  (if (not (`self.Possition Locked`))
    (bind _asbp_game_instance (cast `/Game/GameMode/bp_GameInstance` (`GameplayStatics.GetGameInstance`)))
    (if (== (`self.Current Card Hand Location`) (`KismetArrayLibrary.Array_Find` (`/Game/GameMode/bp_GameInstance.Player 1's Location in Hand` _asbp_game_instance) (`self.Defult Location`)))
      (`KismetSystemLibrary.MoveComponentTo` (`self.obj_Card`) (`self.Defult Location`) (`self.Rotation`)))))

(event `self.ReceiveBeginPlay`
  (bind _game_instance (`self.Game Instance`))
  (bind _card_instance_id_handler (`/Game/GameMode/bp_GameInstance.Card Instance ID Handler` _game_instance))
  ;[1 1 1] Fresh Spawn
  (bind _asbp_game_instance (cast `/Game/GameMode/bp_GameInstance` (`GameplayStatics.GetGameInstance`)))
  (set `self.In Hand` true)
  (bind _output_get (set `self.Game Instance` _asbp_game_instance))
  (set `self.P1 User Interface` (`/Game/GameMode/bp_GameInstance.P1 UserInterface` _asbp_game_instance))
  (set `self.Board` (`/Game/GameMode/bp_GameInstance.Board` _output_get))
  (switch `int` 0
    (:`0`
      (set `self.Player` (`/Game/GameMode/bp_GameInstance.Player 1` _output_get))
      (add `self.Que First/Only Card in Hand (Spawn)` (delegate `Trigger First/Only Card in Hand (Spawn)`))
      (add `self.Que Shift (Card Added)` (delegate `Trigger Shift (Card Added)`))
      (bind _asbp_player (cast `/Game/Blueprints/Players/bp_player` (`self.Player`)))
      (add `/Game/Blueprints/Players/bp_player.Que Shift (Card Added to Hand)` _asbp_player (delegate `Trigger Shift (Added Card)`))
      (add `/Game/Blueprints/Players/bp_player.Move Card in Hand` _asbp_player (delegate `Tirgger Move to New Hand Location`))
      (set `self.Card Instance ID ` _card_instance_id_handler)
      (set `/Game/GameMode/bp_GameInstance.Card Instance ID Handler` (+ _card_instance_id_handler 1) _game_instance))))

(event `Tirgger Move to New Hand Location`
  (params (`Empty Slot` :type Integer) (`Card to Move` :type Integer))
  ;[1 1 1] Fresh Spawn
  (set `self.Current Card Hand Location` `Empty Slot`)
  (`self.Move Card in Hand`))

(event `Trigger First/Only Card in Hand (Spawn)`
  ;[1 1 1] Fresh Spawn
  (`self.First/Only Card in Hand (Spawn)`))

(event `Trigger Shift (Card Added)`
  ;[1 1 1] Fresh Spawn
  (`self.Shift (CardAdded)`))

(event `Trigger Shift (Added Card)`
  ;[1 1 1] Fresh Spawn
  (`self.Shift (CardAdded)`))

(event `self.ReceiveActorOnClicked`
  (params (ButtonPressed :type "Key Structure"))
  (bind _button_1 (`/Game/Blueprints/Huds/bp_p1_UI.Button_1` (`self.P1 User Interface`)))
  ;[1 1 1] Card Options Menu and Set Play Card Event
  (if (`self.In Motion`)
    _
    (elif (not (`self.Possition Locked`))
      (bind _returnvalue (`WidgetLayoutLibrary.GetMousePositionOnViewport`))
      (`Widget.SetRenderTransform` _button_1 (make `WidgetTransform` (`KismetMathLibrary.MakeVector2D` (- (`KismetMathLibrary.BreakVector2D` _returnvalue) 90.0) (- (`.Y` (`KismetMathLibrary.BreakVector2D` _returnvalue)) 50.0))))
      (`Widget.SetVisibility` _button_1 "Visible")
      (bind _asbp_game_instance (cast `/Game/GameMode/bp_GameInstance` (`GameplayStatics.GetGameInstance`)))
      (bind _returnvalue_2 (`KismetArrayLibrary.Array_Find` (`/Game/GameMode/bp_GameInstance.Player 1's Location in Hand` _asbp_game_instance) (`self.Defult Location`)))
      (set `/Game/Blueprints/Huds/bp_p1_UI.Selected Card` (`|GetArrayItem` (`/Game/GameMode/bp_GameInstance.P1 Hand (Game Incstance)` _asbp_game_instance) _returnvalue_2) (`self.P1 User Interface`))
      (set `/Game/Blueprints/Huds/bp_p1_UI.P1 Hand Slot #` _returnvalue_2 (`self.P1 User Interface`))
      (add `/Game/Blueprints/Huds/bp_p1_UI.Button Pressed` (`self.P1 User Interface`) (delegate `Que Play Card`)))))

(event `Que Play Card`
  (params (Object :type "Actor Object Reference") (`Current Card` :type "Actor Class Reference") (`Hand Slot #` :type Integer))
  ;[1 1 1] Card Options Menu and Set Play Card Event
  (bind _output_get (set `self.Selected Card` (`KismetArrayLibrary.Array_Find` (`/Game/GameMode/bp_GameInstance.Player 1's Location in Hand` (stale `self.ReceiveActorOnClicked` _asbp_game_instance)) (`self.Defult Location`))))
  (if (== _output_get `Hand Slot #`)
    (set `self.In Motion` true)
    (add `self.Play Card Dispatcher` (delegate `Play Card`))
    (`self.Play Card`)))

(event `Play Card`
  ;[1 1 1] Card Options Menu and Set Play Card Event
)

(event `First/Only Card in Hand (Spawn)`
  ;[1 1 1] Moving card to Starting/Inital Hand Location
  (bind _asbp_player (cast `/Game/Blueprints/Players/bp_player` (`self.Player`)))
  (set `self.Defult Location` (`/Game/Blueprints/Players/bp_player.Defult Hand Location (Starting) ` _asbp_player))
  (`self.SetActorScale3D` (0.9 0.9 0.9))
  (`KismetSystemLibrary.MoveComponentTo` (`self.obj_Card`) (`self.Defult Location`) (`self.Rotation`))
  (`KismetSystemLibrary.PrintString` "run"))

(event `Shift (CardAdded)`
  (bind _shift__card_added_ (`self.Shift (Card Added)`))
  ;[1 1 1] Where to Move When a Card is Added to Hand
  (set `self.Defult Location` (+ (`self.Defult Location`) _shift__card_added_))
  (`KismetSystemLibrary.PrintString` (`KismetStringLibrary.Conv_VectorToString` (0.0 0.0 0.0)) true true (struct :`R` 1.0 :`G` 0.428499 :`A` 1.0) 5.0)
  (`KismetSystemLibrary.MoveComponentTo` (`self.obj_Card`) _shift__card_added_ (`self.Rotation`) false false 0.6))

(event `self.ReceiveTick`
  (params (DeltaSeconds :type "Float (single-precision)")))

(fn `UserConstructionScript`)