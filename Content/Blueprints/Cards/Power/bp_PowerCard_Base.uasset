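; Base Blueprint for power cards, providing the action that plays a card onto Player 1's power slot on the board.
; PlayCard casts the Board reference to bp_board and, if that slot is already occupied, only clears InMotion.
; Otherwise it marks the slot occupied, resets actor scale and tweens the card component to the slot with a roll rotation, offsetting the target by its displacement from DefultLocation.
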(event `self.Play Card`
  ;[1 1 1] Move to Board
  (bind _asbp_board (cast `/Game/Blueprints/BaseActors/bp_board` (`self.Board`)))
  (if (`/Game/Blueprints/BaseActors/bp_board.P1 POslot Space Occupied` _asbp_board)
    (set `self.In Motion` false)
    (else
      (set `/Game/Blueprints/BaseActors/bp_board.P1 POslot Space Occupied` true _asbp_board)
      (`self.SetActorScale3D` (1.0 1.0 1.0))
      (`KismetSystemLibrary.MoveComponentTo` (`self.obj_Card`) (- (`SceneComponent.K2_GetComponentLocation` (`/Game/Blueprints/BaseActors/bp_board.obj_p1_PowerSlot` _asbp_board)) (- (`SceneComponent.K2_GetComponentLocation` (`self.obj_Card`)) (`self.Defult Location`))) (struct :`Yaw` 180.0) false false 0.3))))

(fn `UserConstructionScript`
  (`parent.UserConstructionScript`))