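; Base Blueprint for equip cards, handling the move of a card onto player 1's side of the board when played.
; PlayCard checks the board for a free equip slot, resets the actor's scale and animates the card object to that slot's stored transform with a fixed yaw.
; It then updates the card's default location, increments the board's slot counter and locks the card's position.
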(event `self.Play Card`
  ;[1 1 1] Move to Board
  (bind _asbp_board (cast `/Game/Blueprints/BaseActors/bp_board` (`self.Board`)))
  (bind _p1_equip_card_slot_on_board (`/Game/Blueprints/BaseActors/bp_board.P1 Equip Card Slot on Board` _asbp_board))
  (if (< _p1_equip_card_slot_on_board 12)
    (`self.SetActorScale3D` (1.0 1.0 1.0))
    (bind _output (`|GetArrayItem` (`/Game/Blueprints/BaseActors/bp_board.P1 EquipCardLocations` _asbp_board) _p1_equip_card_slot_on_board))
    (bind _returnvalue (- (.location _output) (- (`SceneComponent.K2_GetComponentLocation` (`self.obj_Card`)) (`self.Defult Location`))))
    (`KismetSystemLibrary.MoveComponentTo` (`self.obj_Card`) _returnvalue (`KismetMathLibrary.MakeRotator` (.roll (.rotation _output)) (.pitch (.rotation _output)) 150.0) false false 0.3)
    (set `self.Defult Location` _returnvalue)
    (bind _asbp_board_2 (cast `/Game/Blueprints/BaseActors/bp_board` (`self.Board`)))
    (set `/Game/Blueprints/BaseActors/bp_board.P1 Equip Card Slot on Board` (+ _p1_equip_card_slot_on_board 1) _asbp_board_2)
    (set `self.In Motion` false)
    (set `self.Possition Locked` true)))

(fn `UserConstructionScript`
  (`parent.UserConstructionScript`))