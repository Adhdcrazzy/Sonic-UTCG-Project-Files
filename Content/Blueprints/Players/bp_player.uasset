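; Player 1 actor for a card game that spawns the deck on the board and manages that player's hand.
; BeginPlay registers it with the game instance and binds to the board's hand-reassignment event and the UI draw button.
; Draw spawns a fixed character card class at the deck, updates hand arrays and re-calls itself on a delay, within a cap.
; HandReassignment recursively shifts cards two indices down to fill emptied slots.
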(event `self.ReceiveBeginPlay`
  ;[1 1 1] Spawn Deck
  (bind _asbp_game_instance (cast `/Game/GameMode/bp_GameInstance` (`GameplayStatics.GetGameInstance`)))
  (bind _output_get (set `self.Game Instance` _asbp_game_instance))
  (set `/Game/GameMode/bp_GameInstance.Player 1` self _output_get)
  (bind _output_get_2 (set `/Game/GameMode/bp_GameInstance.Board` (`self.Board`) (`self.Game Instance`)))
  (bind _asbp_board (cast `/Game/Blueprints/BaseActors/bp_board` _output_get_2))
  (bind _output_get_3 (set `self.Board Definitive reffrence` _asbp_board))
  (add `/Game/Blueprints/BaseActors/bp_board.Trigger Hand Re-assignment` _output_get_3 (delegate `Trigger Hand Reassignment`))
  (bind _returnvalue (`|SpawnActorFromClass` "/Game/Blueprints/BaseActors/bp_deck.bp_deck_C" (`KismetMathLibrary.MakeTransform` (`SceneComponent.K2_GetComponentLocation` (`/Game/Blueprints/BaseActors/bp_board.obj_p1_DeckSlot` _asbp_board))) "Undefined" "OverrideRootScale" null null))
  (bind _output_get_4 (set `self.Deck` _returnvalue))
  (set `self.Deck Location` (`SceneComponent.K2_GetComponentLocation` (`/Game/Blueprints/BaseActors/bp_deck.obj_deck` _output_get_4)))
  (add `/Game/Blueprints/Huds/bp_p1_UI.Draw Button Pressed` (`/Game/GameMode/bp_GameInstance.P1 UserInterface` (`self.Game Instance`)) (delegate `Que Draw`)))

(event `Trigger Hand Reassignment`
  (params (`Empty Slot` :type Integer))
  ;[1 1 1] Spawn Deck
  (`self.Hand Reassignment` `Empty Slot`))

(event `Que Draw`
  ;[1 1 1] Spawn Deck
  (`self.Draw`))

(event `Hand Reassignment`
  (params (`Empty Slot` :type Integer))
  ;[1 1 1] Re-Arrange Hand After card has been played
  ;;[1 1 1] Check if there are cards to be moved
  (bind _output_get (set `self.Empty Slot` `Empty Slot`))
  (if (<= _output_get (- (`KismetArrayLibrary.Array_LastIndex` (`/Game/GameMode/bp_GameInstance.P1 Hand (Game Incstance)` (`self.Game Instance`))) 2))
    ;;[1 1 1] Determin Card What Card to Move
    (set `self.Card to Move` (+ _output_get 2))
    (bind _outactors (`GameplayStatics.GetAllActorsOfClass` (`|GetArrayItem` (`/Game/GameMode/bp_GameInstance.P1 Hand (Game Incstance)` (`self.Game Instance`)) (`self.Card to Move`))))
    ;;[1 1 1] Select the Right Card (If Multiplule Copies)
    (for _array_element _outactors
      (bind _asbp_card (cast `/Game/Blueprints/BaseActors/bp_Card` _array_element))
      (if (== (`self.Card to Move`) (`KismetArrayLibrary.Array_Find` (`/Game/GameMode/bp_GameInstance.Player 1's Location in Hand` (`self.Game Instance`)) (`/Game/Blueprints/BaseActors/bp_Card.Defult Location` _asbp_card)))
        (set `self.Card in Hand to Move` _array_element)))
    ;;[1 1 1] Move Selected Card in Hand
    (bind _asbp_card_2 (cast `/Game/Blueprints/BaseActors/bp_Card` (`self.Card in Hand to Move`)))
    (set `/Game/Blueprints/BaseActors/bp_Card.Defult Location` (`|GetArrayItem` (`/Game/GameMode/bp_GameInstance.Player 1's Location in Hand` (`self.Game Instance`)) (`self.Empty Slot`)) _asbp_card_2)
    (`self.Move Card in Hand` (`self.Empty Slot`) (`self.Card to Move`))
    ;;[1 1 1] Swap Empty Location and Re-Run Script
    (`KismetArrayLibrary.Array_Swap` (`/Game/GameMode/bp_GameInstance.P1 Hand (Game Incstance)` (`self.Game Instance`)) (`self.Card to Move`) (`self.Empty Slot`))
    (set `self.Empty Slot` (`self.Card to Move`))
    (`self.Hand Reassignment` (`self.Empty Slot`))))

(event `Draw`
  ;[1 1 1] Draw Cardand Set Hand Variables
  ;;[1 1 1] Can Draw
  (if (`self.Draw In Progess`)
    _
    (elif (< (`self.Intial Draw`) 7)
      (set `self.Intial Draw` (+ (`self.Intial Draw`) 1))
      (set `self.Draw In Progess` true)
      ;;[1 1 1] Check if First Card
      (if (`self.First Card`)
        ;;[1 1 1] Set First Card Locarion
        (bind _returnvalue (`KismetArrayLibrary.Array_Add` (`/Game/GameMode/bp_GameInstance.Player 1's Location in Hand` (`self.Game Instance`)) (- (`SceneComponent.K2_GetComponentLocation` (`self.obj_p1_HandSlot_1`)) (`self.Deck Location`))))
        (set `/Game/GameMode/bp_GameInstance.Player 1's Active Slot in Hand` _returnvalue (`self.Game Instance`)))
      ;;[1 1 1] Pick and Spawn Card (Top of Deck)
      (bind _returnvalue_2 (`|SpawnActorFromClass` "/Game/Blueprints/Cards/Character/bp_CharacterCard_1.bp_CharacterCard_1_C" (`KismetMathLibrary.MakeTransform` (+ (0.0 0.0 1.0) (`self.Deck Location`))) "Undefined" "OverrideRootScale" null null))
      ;;[1 1 1] Add to Hand Arrays
      (bind _output_get (set `self.Spawned Card` _returnvalue_2))
      (bind _returnvalue_3 (`GameplayStatics.GetObjectClass` _output_get))
      (`KismetArrayLibrary.Array_Add` (`self.P1 Hand (Player)`) _returnvalue_3)
      (`KismetArrayLibrary.Array_Add` (`/Game/GameMode/bp_GameInstance.P1 Hand (Game Incstance)` (`self.Game Instance`)) _returnvalue_3)
      ;;[1 1 1] Check if First Card in Hand
      (if (not (`self.Is First Card in Hand`))
        ;;[1 1 1] Inital Hand Controller
        (`self.Que Shift (Card Added to Hand)`))
      (set `self.Defult Hand Location (Starting) ` (- (`SceneComponent.K2_GetComponentLocation` (`self.obj_p1_HandSlot_1`)) (`self.Deck Location`)))
      (set `self.Is First Card in Hand` false)
      (`/Game/Blueprints/BaseActors/bp_Card.Que First/Only Card in Hand (Spawn)` (`self.Spawned Card`))
      ;;[1 1 1] Re-assign Veriables
      (set `self.Draw In Progess` false)
      (set `self.First Card` false)
      (`self.Que Equip Card Event`)
      ;;[1 1 1] Inital Draw Regulator
      (if (not (== (`self.Intial Draw`) 2))
        (`KismetSystemLibrary.Delay` 1.0)
        (`self.Draw`)))))

(fn `UserConstructionScript`)